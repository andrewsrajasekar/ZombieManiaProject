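; Shotgun weapon Blueprint that extends a parent weapon class with shotgun-specific ammo, reload timing and firing effects.
; On BeginPlay it pulls shotgun ammo data from the ZombieMania game instance, then sets reload time in proportion to magazine capacity.
; Firing runs the parent logic, then plays the gun mesh fire animation and spawns a shell-ejection particle at the AmmoEject socket.
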(event Custom|SetReloadTime
  (Variables|Default|SetReloadTime (* (Variables|Default|GetMaxMagAmmo) 0.5)))

(event EventBeginPlay
  (|CallParentFunction)
  (bind _aszombie_mania_game_instance (Utilities|Casting|CastToZombieMania_GameInstance (Game|GetGameInstance)))
  (Variables|Default|SetAmmoData (Variables|/Game/BluePrints/ZombieMania_GameInstance.ZombieMania_GameInstance_C|GetShotGunAmmoData _aszombie_mania_game_instance))
  (CallFunction|SetReloadTime))

(event EventWeaponFire
  (params (FireType :type FireTypes%20Enum :default "NewEnumerator0"))
  (bind _gunmesh (Variables|Default|GetGunMesh))
  (bind _returnvalue (Transformation|GetSocketTransform _gunmesh "AmmoEject" "RTS_World"))
  (|CallParentFunction FireType)
  (Components|Animation|PlayAnimation _gunmesh "/Game/MilitaryWeapSilver/Weapons/Animations/Fire_Shotgun_W.Fire_Shotgun_W" false)
  (Effects|SpawnEmitteratLocation "/Game/Particles/FX_ShotGunShell.FX_ShotGunShell" (.location _returnvalue) (.rotation _returnvalue)))

(fn ConstructionScript
  (|CallParentFunction))