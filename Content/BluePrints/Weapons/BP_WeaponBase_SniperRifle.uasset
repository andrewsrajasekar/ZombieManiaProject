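; Sniper rifle weapon for ZombieMania, extending a base weapon and loading its ammo data from the game instance on BeginPlay.
; Firing plays the gun animation, then applies controller recoil while aiming or spawns a shell-eject effect when hip-firing.
; Aiming locks switching and reloading, then after a brief delay shows the scope widget, hides gun, player and HUD, and zeroes bullet spread.
; Exiting aim restores them.
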(event EventBeginPlay
  (|CallParentFunction)
  (bind _aszombie_mania_game_instance (Utilities|Casting|CastToZombieMania_GameInstance (Game|GetGameInstance)))
  (Variables|Default|SetAmmoData (Variables|/Game/BluePrints/ZombieMania_GameInstance.ZombieMania_GameInstance_C|GetSniperRifleAmmoData _aszombie_mania_game_instance)))

(event Collision|EventActorBeginOverlap
  (params (OtherActor :type Actor%20Object%20Reference))
  (|CallParentFunction OtherActor) ; This node is disabled and will not be called.\nDrag off pins to build functionality.
)

(event EventTick
  (params (DeltaSeconds :type Float%20%28single-precision%29))
  (|CallParentFunction DeltaSeconds) ; This node is disabled and will not be called.\nDrag off pins to build functionality.
)

(event EventWeaponFire
  (params (FireType :type FireTypes%20Enum :default "NewEnumerator0"))
  (bind _gunmesh (Variables|Default|GetGunMesh))
  (bind _returnvalue (Transformation|GetSocketTransform _gunmesh "AmmoEject" "RTS_World"))
  (|CallParentFunction FireType)
  (Components|Animation|PlayAnimation (Variables|Default|GetGunMesh) "/Game/MilitaryWeapSilver/Weapons/Animations/Fire_SniperRifle_W.Fire_SniperRifle_W" false)
  (if (Variables|Default|GetisAiming)
    (CallFunction|ControllerInputRecoil)
    (else
      (Effects|SpawnEmitteratLocation "/Game/Particles/FX_SniperRifleShell.FX_SniperRifleShell" (.location _returnvalue) (.rotation _returnvalue)))))

(event EventOnAimEnter
  (bind _playerref (Variables|Default|GetPlayerRef))
  (bind _playerref_2 (Variables|Default|GetPlayerRef))
  (bind _sniperscoperef (Variables|/Game/BluePrints/ZombieMania_Character.ZombieMania_Character_C|GetSniperScopeRef _playerref))
  (|CallParentFunction)
  (if (== (Variables|/Game/BluePrints/ZombieMania_Character.ZombieMania_Character_C|GetCurrentWeapon (Variables|Default|GetPlayerRef)) self)
    (Variables|/Game/BluePrints/ZombieMania_Character.ZombieMania_Character_C|SetCanSwitchWeapon _playerref_2 false)
    (Variables|/Game/BluePrints/ZombieMania_Character.ZombieMania_Character_C|SetCanReload _playerref_2 false)
    (Utilities|FlowControl|Delay 0.1) ; This Delay is added to Pull up Sniper to Eye
    (if (not (UserInterface|Viewport|IsinViewport _sniperscoperef))
      (UserInterface|Viewport|AddtoViewport _sniperscoperef 0)
      (Development|SetHiddeninGame (Variables|Default|GetGunMesh) true false)
      (Rendering|SetActorHiddenInGame (Game|Player|GetPlayerPawn 0) true)
      (Widget|SetVisibility (Variables|/Game/BluePrints/ZombieMania_Character.ZombieMania_Character_C|GetMainHUDRef (Variables|Default|GetPlayerRef)) "Collapsed")
      (Variables|Default|SetBulletSpread 0.0))))

(event EventOnAimExit
  (bind _playerref (Variables|Default|GetPlayerRef))
  (|CallParentFunction)
  (Variables|/Game/BluePrints/ZombieMania_Character.ZombieMania_Character_C|SetCanSwitchWeapon _playerref true)
  (Variables|/Game/BluePrints/ZombieMania_Character.ZombieMania_Character_C|SetCanReload _playerref true)
  (Widget|RemovefromParent (Variables|/Game/BluePrints/ZombieMania_Character.ZombieMania_Character_C|GetSniperScopeRef _playerref))
  (Development|SetHiddeninGame (Variables|Default|GetGunMesh) false false)
  (Rendering|SetActorHiddenInGame (Game|Player|GetPlayerPawn 0) false)
  (Widget|SetVisibility (Variables|/Game/BluePrints/ZombieMania_Character.ZombieMania_Character_C|GetMainHUDRef (Variables|Default|GetPlayerRef)) "Visible")
  (Variables|Default|SetBulletSpread 8e+02))

(fn ConstructionScript
  (|CallParentFunction))