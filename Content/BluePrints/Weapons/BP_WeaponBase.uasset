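; Base weapon for the ZombieMania player, handling firing, magazine and reserve ammo, reloads and recoil.
; WeaponFire uses CalculateShot's camera trace, with random spread unless aiming, for hitscan shots or projectiles launched from the muzzle toward the hit point.
; Hitscan spawns trail and impact effects and sends damage by message, while projectiles receive the ammo data.
; Automatic weapons play a timeline recoil that kicks controller pitch and yaw, and Tick drives the player's ADS FOV.
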(event Custom|ControllerInputRecoil
  (bind _returnvalue (Game|Player|GetPlayerPawn 0))
  (bind (_direction _alpha) (Timeline|RecoilTimeline PlayFromStart)
    (:Update
      (switch Utilities|FlowControl|Switch|SwitchonETimelineDirection _direction
        (:Forward
          (Pawn|Input|AddControllerPitchInput _returnvalue (Math|Float|Lerp 0.0 (Variables|Recoil|GetRecoilPitch) _alpha))
          (Pawn|Input|AddControllerYawInput _returnvalue (Math|Random|RandomFloatinRange -0.15 0.15)))
        (:Backward
          (Pawn|Input|AddControllerPitchInput _returnvalue (* (Math|Float|Lerp 0.0 (Variables|Recoil|GetRecoilPitch) _alpha) -1.0)))))
    (:Finished
      (CallFunction|ReverseRecoil)
      (Utilities|FlowControl|RetriggerableDelay 0.01)
      (CallFunction|StopRecoil))))

(event Custom|StopRecoil
  (bind _returnvalue (Game|Player|GetPlayerPawn 0))
  (bind (_direction _alpha) (Timeline|RecoilTimeline Stop)
    (:Update
      (switch Utilities|FlowControl|Switch|SwitchonETimelineDirection _direction
        (:Forward
          (Pawn|Input|AddControllerPitchInput _returnvalue (Math|Float|Lerp 0.0 (Variables|Recoil|GetRecoilPitch) _alpha))
          (Pawn|Input|AddControllerYawInput _returnvalue (Math|Random|RandomFloatinRange -0.15 0.15)))
        (:Backward
          (Pawn|Input|AddControllerPitchInput _returnvalue (* (Math|Float|Lerp 0.0 (Variables|Recoil|GetRecoilPitch) _alpha) -1.0)))))
    (:Finished
      (CallFunction|ReverseRecoil)
      (Utilities|FlowControl|RetriggerableDelay 0.01)
      (CallFunction|StopRecoil))))

(event Custom|ReverseRecoil
  (bind _returnvalue (Game|Player|GetPlayerPawn 0))
  (bind (_direction _alpha) (Timeline|RecoilTimeline Reverse)
    (:Update
      (switch Utilities|FlowControl|Switch|SwitchonETimelineDirection _direction
        (:Forward
          (Pawn|Input|AddControllerPitchInput _returnvalue (Math|Float|Lerp 0.0 (Variables|Recoil|GetRecoilPitch) _alpha))
          (Pawn|Input|AddControllerYawInput _returnvalue (Math|Random|RandomFloatinRange -0.15 0.15)))
        (:Backward
          (Pawn|Input|AddControllerPitchInput _returnvalue (* (Math|Float|Lerp 0.0 (Variables|Recoil|GetRecoilPitch) _alpha) -1.0)))))
    (:Finished
      (CallFunction|ReverseRecoil)
      (Utilities|FlowControl|RetriggerableDelay 0.01)
      (CallFunction|StopRecoil))))

(event Custom|OnAimEnter
  (Variables|ADS|SetisAiming true))

(event Custom|OnAimExit
  (Variables|ADS|SetisAiming false))

(event EventBeginPlay
  (bind _aszombie_mania_character (Utilities|Casting|CastToZombieMania_Character (Game|Player|GetPlayerPawn 0)))
  (Variables|References|SetPlayerRef _aszombie_mania_character)
  (EventDispatchers|AssignAimEnter _aszombie_mania_character (delegate Custom|OnAimEnter))
  (EventDispatchers|AssignAimExit _aszombie_mania_character (delegate Custom|OnAimExit)))

(event EventTick
  (params (DeltaSeconds :type Float%20%28single-precision%29))
  (Default|ADSFOV (Variables|References|GetPlayerRef)))

(fn ConstructionScript)

(fn WeaponFire
  (params (FireType :type FireTypes%20Enum :default "NewEnumerator0"))
  (Variables|Ammo|SetCurrentAmmo (- (Variables|Ammo|GetCurrentAmmo) 1))
  (switch Utilities|FlowControl|Switch|SwitchonFireTypes FireType
    (:NewEnumerator0
      (if (Variables|Ammo|GetmultipleBullets)
        (for _index (range 0 (- (Variables|Ammo|GetBulletCount) 1))
          (bind (_hitresult _projectiletransform _endlocation) (CallFunction|CalculateShot (Variables|/Game/BluePrints/ZombieMania_Character.ZombieMania_Character_C|GetCamera (Variables|References|GetPlayerRef)) (Variables|Default|GetGunMesh) "MuzzleFlash"))
          (bind _returnvalue (Effects|SpawnEmitteratLocation (Variables|Properties|GetTrailFX) (Transformation|GetSocketLocation (Variables|Default|GetGunMesh) "MuzzleFlash")))
          (Effects|Components|ParticleSystem|SetVectorParameter _returnvalue "ShockBeamEnd" _endlocation)
          (Game|SpawnActorfromClass (Variables|Properties|GetImpactEffectClass) (Math|Transform|MakeTransform (.ImpactPoint (Collision|BreakHitResult _hitresult)) "0, 0, 0" "1,1,1") "Undefined" 0 _hitresult (.bBlockingHit (Collision|BreakHitResult _hitresult)) 0)
          (CallFunction|AddDamage _hitresult)
          (if (Variables|Properties|GetisAutomaticWeapon)
            (CallFunction|ControllerInputRecoil)))
        (else
          (bind (_hitresult_2 _projectiletransform_2 _endlocation_2) (CallFunction|CalculateShot (Variables|/Game/BluePrints/ZombieMania_Character.ZombieMania_Character_C|GetCamera (Variables|References|GetPlayerRef)) (Variables|Default|GetGunMesh) "MuzzleFlash"))
          (bind _returnvalue_2 (Effects|SpawnEmitteratLocation (Variables|Properties|GetTrailFX) (Transformation|GetSocketLocation (Variables|Default|GetGunMesh) "MuzzleFlash")))
          (Effects|Components|ParticleSystem|SetVectorParameter _returnvalue_2 "ShockBeamEnd" _endlocation_2)
          (Game|SpawnActorfromClass (Variables|Properties|GetImpactEffectClass) (Math|Transform|MakeTransform (.ImpactPoint (Collision|BreakHitResult _hitresult_2)) "0, 0, 0" "1,1,1") "Undefined" 0 _hitresult_2 (.bBlockingHit (Collision|BreakHitResult _hitresult_2)) 0)
          (CallFunction|AddDamage _hitresult_2)
          (if (Variables|Properties|GetisAutomaticWeapon) :!label _label
            (CallFunction|ControllerInputRecoil)))))
    (:NewEnumerator1
      (bind _projectiletransform_3 (CallFunction|CalculateShot (Variables|/Game/BluePrints/ZombieMania_Character.ZombieMania_Character_C|GetCamera (Variables|References|GetPlayerRef)) (Variables|Default|GetGunMesh) "MuzzleFlash"))
      (bind _returnvalue_3 (Game|SpawnActorfromClass (Variables|Projectile|GetProjectile) _projectiletransform_3 "AlwaysSpawn" 0 (Variables|Properties|GetAmmoData) (Variables|Stats|GetCriticalHitDamageModifier) 0))
      (Variables|Projectile|SetSpawnedProjectile _returnvalue_3)
      (goto _label))))

(fn WeaponReload
  (LocalVariables|SetAmmoNeededForFullMag (- (Variables|Ammo|GetMaxMagAmmo) (Variables|Ammo|GetCurrentAmmo)))
  (if (> (Variables|Ammo|GetCurrentTotalAmmo) (LocalVariables|GetAmmoNeededForFullMag))
    (Variables|Ammo|SetCurrentTotalAmmo (- (Variables|Ammo|GetCurrentTotalAmmo) (LocalVariables|GetAmmoNeededForFullMag)))
    (Variables|Ammo|SetCurrentAmmo (Variables|Ammo|GetMaxMagAmmo))
    (else
      (Variables|Ammo|SetCurrentAmmo (+ (Variables|Ammo|GetCurrentTotalAmmo) (Variables|Ammo|GetCurrentAmmo)))
      (Variables|Ammo|SetCurrentTotalAmmo 0))))

(fn HasAmmoinMag
  (return (> (Variables|Ammo|GetCurrentAmmo) 0) (== (Variables|Ammo|GetCurrentAmmo) (Variables|Ammo|GetMaxMagAmmo))))

(fn HasExtraAmmo
  (return (> (Variables|Ammo|GetCurrentTotalAmmo) 0)))

(fn CalculateShot
  (params (Camera :type Camera%20Component%20Object%20Reference) (WeaponeMesh :type Scene%20Component%20Object%20Reference) (WeaponFireSocketName :type Name))
  (bind _bulletspread (Variables|Stats|GetBulletSpread))
  (bind _returnvalue (* _bulletspread -1.0))
  (Utilities|FlowControl|Sequence
    (:then_0
      (LocalVariables|SetLocalCamera Camera)
      (LocalVariables|SetLocalWeaponMesh WeaponeMesh)
      (LocalVariables|SetLocalSocketName WeaponFireSocketName))
    (:then_1
      (LocalVariables|SetLocalEndLocation (select (Variables|ADS|GetisAiming) (+ (.location (Transformation|GetWorldTransform (LocalVariables|GetLocalCamera))) (* (Math|Vector|GetForwardVector (.rotation (Transformation|GetWorldTransform (LocalVariables|GetLocalCamera)))) (Variables|Stats|GetBulletSpreadMultiplier))) (Math|Vector|MakeVector (+ (.X (Math|Vector|BreakVector (+ (.location (Transformation|GetWorldTransform (LocalVariables|GetLocalCamera))) (* (Math|Vector|GetForwardVector (.rotation (Transformation|GetWorldTransform (LocalVariables|GetLocalCamera)))) (Variables|Stats|GetBulletSpreadMultiplier))))) (Math|Random|RandomFloatinRange _returnvalue _bulletspread)) (+ (.Y (Math|Vector|BreakVector (+ (.location (Transformation|GetWorldTransform (LocalVariables|GetLocalCamera))) (* (Math|Vector|GetForwardVector (.rotation (Transformation|GetWorldTransform (LocalVariables|GetLocalCamera)))) (Variables|Stats|GetBulletSpreadMultiplier))))) (Math|Random|RandomFloatinRange _returnvalue _bulletspread)) (+ (.Z (Math|Vector|BreakVector (+ (.location (Transformation|GetWorldTransform (LocalVariables|GetLocalCamera))) (* (Math|Vector|GetForwardVector (.rotation (Transformation|GetWorldTransform (LocalVariables|GetLocalCamera)))) (Variables|Stats|GetBulletSpreadMultiplier))))) (Math|Random|RandomFloatinRange _returnvalue _bulletspread)))))
      (bind (_outhit _returnvalue_2) (Collision|LineTraceForObjects (.location (Transformation|GetWorldTransform (LocalVariables|GetLocalCamera))) (select (Variables|ADS|GetisAiming) (+ (.location (Transformation|GetWorldTransform (LocalVariables|GetLocalCamera))) (* (Math|Vector|GetForwardVector (.rotation (Transformation|GetWorldTransform (LocalVariables|GetLocalCamera)))) (Variables|Stats|GetBulletSpreadMultiplier))) (Math|Vector|MakeVector (+ (.X (Math|Vector|BreakVector (+ (.location (Transformation|GetWorldTransform (LocalVariables|GetLocalCamera))) (* (Math|Vector|GetForwardVector (.rotation (Transformation|GetWorldTransform (LocalVariables|GetLocalCamera)))) (Variables|Stats|GetBulletSpreadMultiplier))))) (Math|Random|RandomFloatinRange _returnvalue _bulletspread)) (+ (.Y (Math|Vector|BreakVector (+ (.location (Transformation|GetWorldTransform (LocalVariables|GetLocalCamera))) (* (Math|Vector|GetForwardVector (.rotation (Transformation|GetWorldTransform (LocalVariables|GetLocalCamera)))) (Variables|Stats|GetBulletSpreadMultiplier))))) (Math|Random|RandomFloatinRange _returnvalue _bulletspread)) (+ (.Z (Math|Vector|BreakVector (+ (.location (Transformation|GetWorldTransform (LocalVariables|GetLocalCamera))) (* (Math|Vector|GetForwardVector (.rotation (Transformation|GetWorldTransform (LocalVariables|GetLocalCamera)))) (Variables|Stats|GetBulletSpreadMultiplier))))) (Math|Random|RandomFloatinRange _returnvalue _bulletspread)))) (Utilities|Array|MakeArray "ObjectTypeQuery1" "ObjectTypeQuery2") false (Utilities|Array|MakeArray (Game|Player|GetPlayerPawn 0)) "None"))
      (if _returnvalue_2
        (LocalVariables|SetLocalProjectileTransform (Math|Transform|MakeTransform (Transformation|GetSocketLocation (LocalVariables|GetLocalWeaponMesh) (LocalVariables|GetLocalSocketName)) (Math|Rotator|FindLookatRotation (Transformation|GetSocketLocation (LocalVariables|GetLocalWeaponMesh) (LocalVariables|GetLocalSocketName)) (.ImpactPoint (Collision|BreakHitResult _outhit)))))
        (LocalVariables|SetLocalEndLocation (.ImpactPoint (Collision|BreakHitResult _outhit)))
        (else
          (LocalVariables|SetLocalProjectileTransform (Math|Transform|MakeTransform (Transformation|GetSocketLocation (LocalVariables|GetLocalWeaponMesh) (LocalVariables|GetLocalSocketName)) (Pawn|GetControlRotation (.AsPawn (Utilities|Casting|CastToPawn (Components|GetOwner (LocalVariables|GetLocalCamera)))) :!class /Script/Engine.Pawn))))))
    (:then_2
      (return _outhit (LocalVariables|GetLocalProjectileTransform) (LocalVariables|GetLocalEndLocation)))))

(fn AddDamage
  (params (HitResult :type Hit%20Result%20Structure))
  (Class|TakeDamage|TakeDamage(Message) (.HitActor (Collision|BreakHitResult HitResult)) (Variables|Properties|GetAmmoData) (Variables|Stats|GetCriticalHitDamageModifier) HitResult))

(fn StopFire)