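; Grenade launcher weapon Blueprint for ZombieMania, extending a parent weapon class.
; On BeginPlay it takes its ammo data from the grenade launcher entry in the game instance.
; On firing it runs the parent fire logic, plays the launcher's mesh fire animation and triggers a world camera shake at its location, reusing the rocket launcher's shake.
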(event EventBeginPlay
  (|CallParentFunction)
  (bind _aszombie_mania_game_instance (Utilities|Casting|CastToZombieMania_GameInstance (Game|GetGameInstance)))
  (Variables|Default|SetAmmoData (Variables|/Game/BluePrints/ZombieMania_GameInstance.ZombieMania_GameInstance_C|GetGrenadeLauncherAmmoData _aszombie_mania_game_instance)))

(event EventWeaponFire
  (params (FireType :type FireTypes%20Enum :default "NewEnumerator0"))
  (|CallParentFunction FireType)
  (Components|Animation|PlayAnimation (Variables|Default|GetGunMesh) "/Game/MilitaryWeapSilver/Weapons/Animations/Fire_GrenadeLauncher_W.Fire_GrenadeLauncher_W" false)
  (Camera|PlayWorldCameraShake "/Game/BluePrints/CameraShakes/RocketLauncher_CameraShake.RocketLauncher_CameraShake_C" (Transformation|GetActorLocation) 0.0 5e+02))

(fn ConstructionScript
  (|CallParentFunction))