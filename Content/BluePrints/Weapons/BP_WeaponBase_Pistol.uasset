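; Pistol weapon Blueprint that extends a parent weapon class with pistol-specific ammo data and firing effects.
; On BeginPlay it sets its AmmoData from PistolAmmoData on the ZombieMania game instance.
; WeaponFire runs the parent logic, then plays the gun mesh fire animation and spawns a shell particle at the AmmoEject socket.
; Reload and construction only call the parent, and the overlap and Tick events are disabled.
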(event EventBeginPlay
  (|CallParentFunction)
  (bind _aszombie_mania_game_instance (Utilities|Casting|CastToZombieMania_GameInstance (Game|GetGameInstance)))
  (Variables|Default|SetAmmoData (Variables|/Game/BluePrints/ZombieMania_GameInstance.ZombieMania_GameInstance_C|GetPistolAmmoData _aszombie_mania_game_instance)))

(event Collision|EventActorBeginOverlap
  (params (OtherActor :type Actor%20Object%20Reference))
  (|CallParentFunction OtherActor) ; This node is disabled and will not be called.\nDrag off pins to build functionality.
)

(event EventTick
  (params (DeltaSeconds :type Float%20%28single-precision%29))
  (|CallParentFunction DeltaSeconds) ; This node is disabled and will not be called.\nDrag off pins to build functionality.
)

(event EventWeaponFire
  (params (FireType :type FireTypes%20Enum :default "NewEnumerator0"))
  (bind _gunmesh (Variables|Default|GetGunMesh))
  (bind _returnvalue (Transformation|GetSocketTransform _gunmesh "AmmoEject" "RTS_World"))
  (|CallParentFunction FireType)
  (Components|Animation|PlayAnimation (Variables|Default|GetGunMesh) "/Game/MilitaryWeapSilver/Weapons/Animations/Fire_Pistol_W.Fire_Pistol_W" false)
  (Effects|SpawnEmitteratLocation "/Game/Particles/FX_PistolShell.FX_PistolShell" (.location _returnvalue) (.rotation _returnvalue)))

(event EventWeaponReload
  (|CallParentFunction))

(fn ConstructionScript
  (|CallParentFunction))