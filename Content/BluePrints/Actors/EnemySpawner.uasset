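; EnemySpawner is a placeable actor that spawns AI zombies in Zombie Mania.
; Its SpawnZombie event creates an AI_Character_Child with AI_BehaviorTree at the spawner's transform and increments the zombie count on the game state.
; Each spawned zombie receives the world location of the StartGoalLocation component as its initial goal.
; The construction script positions that component from per-instance relative location and rotation variables.
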(event Custom|SpawnZombie
  (bind _returnvalue (Transformation|GetActorTransform))
  (bind (_location _rotation) (Math|Transform|BreakTransform _returnvalue))
  (bind _returnvalue_2 (AI|SpawnAIFromClass "/Game/AI/AI_Character_Child.AI_Character_Child_C" "/Game/AI/AI_BehaviorTree.AI_BehaviorTree" _location _rotation true 0))
  (Math|Integer|IncrementInt (Variables|/Game/BluePrints/ZombieMania_GameState.ZombieMania_GameState_C|GetNumberOfZombies (Variables|Default|GetGameStateRef))
    (:%20%20
      (bind _asai_character_child (Utilities|Casting|CastToAI_Character_Child _returnvalue_2))
      (Variables|/Game/AI/AI_Character.AI_Character_C|SetStartGoalLocation _asai_character_child (Transformation|GetWorldLocation (Variables|Default|GetStartGoalLocation))))))

(event EventBeginPlay
  (bind _aszombie_mania_game_state (Utilities|Casting|CastToZombieMania_GameState (Game|GetGameState)))
  (Variables|Default|SetGameStateRef _aszombie_mania_game_state))

(fn ConstructionScript
  (Transformation|SetRelativeLocationAndRotation (Variables|Default|GetStartGoalLocation) (Variables|Default|GetGoalLocationVector) (Variables|Default|GetGoalRotator) false false))