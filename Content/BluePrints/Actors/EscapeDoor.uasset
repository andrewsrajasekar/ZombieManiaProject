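; EscapeDoor is the exit actor that ends a ZombieMania run once all objectives are completed.
; EscapeOnProgress toggles its visibility, and sphere overlap binds the player's interact, reusing the weapon-buy HUD as an escape prompt.
; Interacting destroys AI characters and spawners, shows credits briefly, then pauses into the end-game variant of the game-over screen with player stats and UI-only input.
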(event OnComponentBeginOverlap(Sphere)
  (params (OverlappedComponent :type Primitive%20Component%20Object%20Reference) (OtherActor :type Actor%20Object%20Reference) (OtherComp :type Primitive%20Component%20Object%20Reference) (OtherBodyIndex :type Integer) (bFromSweep :type Boolean) (SweepResult :type Hit%20Result%20Structure%20%28by%20ref%29))
  (bind _isallobjectivescompleted_ (Default|AllObjectivesCompleted (Variables|Default|GetGameStateRef)))
  (if _isallobjectivescompleted_
    (bind _aszombie_mania_character (Utilities|Casting|CastToZombieMania_Character OtherActor))
    (EventDispatchers|AssignInteract _aszombie_mania_character (delegate Custom|Interact))
    (if (UserInterface|Viewport|IsinViewport (Variables|/Game/BluePrints/ZombieMania_Character.ZombieMania_Character_C|GetWeaponBuyHUDRef _aszombie_mania_character))
      (Widget|RemovefromParent (Variables|/Game/BluePrints/ZombieMania_Character.ZombieMania_Character_C|GetWeaponBuyHUDRef _aszombie_mania_character)))
    (UserInterface|Viewport|AddtoViewport (Variables|/Game/BluePrints/ZombieMania_Character.ZombieMania_Character_C|GetWeaponBuyHUDRef _aszombie_mania_character) 0)
    (Default|UpdateData (Variables|/Game/BluePrints/ZombieMania_Character.ZombieMania_Character_C|GetWeaponBuyHUDRef _aszombie_mania_character) "Escape" 0 true)))

(event OnComponentEndOverlap(Sphere)
  (params (OverlappedComponent :type Primitive%20Component%20Object%20Reference) (OtherActor :type Actor%20Object%20Reference) (OtherComp :type Primitive%20Component%20Object%20Reference) (OtherBodyIndex :type Integer))
  (bind _aszombie_mania_character (Utilities|Casting|CastToZombieMania_Character OtherActor))
  (EventDispatchers|UnbindEventfromInteract _aszombie_mania_character (delegate Custom|Interact))
  (Widget|RemovefromParent (Variables|/Game/BluePrints/ZombieMania_Character.ZombieMania_Character_C|GetWeaponBuyHUDRef _aszombie_mania_character)))

(event Custom|Interact
  (bind _returnvalue (Game|GetPlayerController 0))
  (bind _playerstateref (Variables|Default|GetPlayerStateRef))
  (bind _isallobjectivescompleted_ (Default|AllObjectivesCompleted (Variables|Default|GetGameStateRef)))
  (if _isallobjectivescompleted_
    (Variables|/Game/BluePrints/ZombieMania_Character.ZombieMania_Character_C|SetcanGameBePaused (Variables|Default|GetPlayerRef) false)
    (bind _outactors (Actor|GetAllActorsOfClass "/Game/AI/AI_Character_Child.AI_Character_Child_C"))
    (for _array_element _outactors
      (Actor|DestroyActor _array_element))
    (bind _outactors_2 (Actor|GetAllActorsOfClass "/Game/BluePrints/Actors/EnemySpawner.EnemySpawner_C"))
    (for _array_element_2 _outactors_2
      (Actor|DestroyActor _array_element_2))
    (bind _returnvalue_2 (UserInterface|CreateWidget "/Game/BluePrints/UMG/HUD_GameCredits.HUD_GameCredits_C"))
    (UserInterface|Viewport|AddtoViewport _returnvalue_2 0)
    (Utilities|FlowControl|Delay 7.0)
    (Game|SetGamePaused true)
    (Variables|/Game/BluePrints/ZombieMania_Character.ZombieMania_Character_C|SetIsGamePaused (Variables|Default|GetPlayerRef) true)
    (if (UserInterface|Viewport|IsinViewport _returnvalue_2)
      _
      (else
        _))
    (Widget|RemovefromParent _returnvalue_2)
    (bind _returnvalue_3 (UserInterface|CreateWidget "/Game/BluePrints/UMG/HUD_GameOver.HUD_GameOver_C" 0 (Variables|/Game/BluePrints/ZombieMania_PlayerState.ZombieMania_PlayerState_C|GetCurrentPoints _playerstateref) (Variables|/Game/BluePrints/ZombieMania_PlayerState.ZombieMania_PlayerState_C|GetZombiesKilled _playerstateref) (Variables|/Game/BluePrints/ZombieMania_PlayerState.ZombieMania_PlayerState_C|GetAmountOfHeadShots _playerstateref)))
    (bind _output_get (Variables|Default|SetGameOverHUD _returnvalue_3))
    (Default|ChangeWidgettoEndGame _output_get)
    (if (UserInterface|Viewport|IsinViewport (Variables|Default|GetGameOverHUD))
      (Widget|RemovefromParent (Variables|Default|GetGameOverHUD)))
    (UserInterface|Viewport|AddtoViewport (Variables|Default|GetGameOverHUD) 0)
    (Widget|SetVisibility (Variables|/Game/BluePrints/UMG/MainHUD.MainHUD_C|GetUI_DynamicCrosshair (Variables|/Game/BluePrints/ZombieMania_Character.ZombieMania_Character_C|GetMainHUDRef (Variables|Default|GetPlayerRef))) "Collapsed")
    (Input|SetInputModeUIOnly _returnvalue (Variables|Default|GetGameOverHUD) "DoNotLock")
    (Variables|/Script/Engine.PlayerController|SetbShowMouseCursor _returnvalue true)))

(event EventBeginPlay
  (bind _aszombie_mania_game_state (Utilities|Casting|CastToZombieMania_GameState (Game|GetGameState)))
  (Variables|Default|SetGameStateRef _aszombie_mania_game_state)
  (bind _aszombie_mania_player_state (Utilities|Casting|CastToZombieMania_PlayerState (Variables|/Script/Engine.Controller|GetPlayerState (Game|GetPlayerController 0))))
  (Variables|Default|SetPlayerStateRef _aszombie_mania_player_state)
  (bind _aszombie_mania_character (Utilities|Casting|CastToZombieMania_Character (Game|Player|GetPlayerPawn 0)))
  (Variables|Default|SetPlayerRef _aszombie_mania_character))

(fn ConstructionScript)

(fn EscapeonProgress
  (params (allObjectivesCompleted? :type Boolean))
  (bind _defaultsceneroot (Variables|Default|GetDefaultSceneRoot))
  (if allObjectivesCompleted?
    (Rendering|SetVisibility _defaultsceneroot true true)
    (else
      (Rendering|SetVisibility _defaultsceneroot false true))))