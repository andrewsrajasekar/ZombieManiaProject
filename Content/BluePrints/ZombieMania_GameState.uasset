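; Game state for a zombie wave mode that tracks rounds, remaining zombies to spawn and player objectives.
; Rounds scale zombie counts up to a cap and update the HUD, and an empty count makes the game mode start the next round.
; Objectives form a map of progress labels to completion flags, rebuilt before the all-completed check.
; A tiered lookup returns a player damage amount that rises with the round.
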(event EventBeginPlay
  (bind _aszombie_mania_game_mode (Utilities|Casting|CastToZombieMania_GameMode (Game|GetGameMode)))
  (Variables|Default|SetGameModeRef _aszombie_mania_game_mode)
  (bind _aszombie_mania_character (Utilities|Casting|CastToZombieMania_Character (Game|Player|GetPlayerPawn 0)))
  (Variables|Default|SetPlayerRef _aszombie_mania_character)
  (bind _aszombie_mania_player_state (Utilities|Casting|CastToZombieMania_PlayerState (Variables|/Script/Engine.Controller|GetPlayerState (Game|GetPlayerController 0))))
  (Variables|Default|SetPlayerStateRef _aszombie_mania_player_state)
  (CallFunction|AddObjectives))

(event EventTick
  (params (DeltaSeconds :type Float%20%28single-precision%29)))

(fn ConstructionScript)

(fn IncreaseRound
  (Math|Integer|IncrementInt (Variables|Default|GetCurrentRound)
    (:%20%20
      (bind _output_get (Variables|Default|SetNumberOfZombiesToSpawn (Math|Integer|Clamp(Integer) (+ (* (Variables|Default|GetCurrentRound) 2) (* (+ (Variables|Default|GetCurrentRound) 1) 2)) 0 150)))
      (Default|UpdateRoundInfo (Variables|/Game/BluePrints/UMG/MainHUD.MainHUD_C|GetUI_RoundNumber (Variables|/Game/BluePrints/ZombieMania_Character.ZombieMania_Character_C|GetMainHUDRef (Variables|Default|GetPlayerRef))) (Variables|Default|GetCurrentRound) _output_get))))

(fn CheckifRoundIsOver
  (if (<= (Variables|Default|GetNumberOfZombiesToSpawn) 0)
    (Default|StartNewRound (Variables|Default|GetGameModeRef))))

(fn AddObjectives
  (bind _playerstateref (Variables|Default|GetPlayerStateRef))
  (bind _currentpoints (Variables|/Game/BluePrints/ZombieMania_PlayerState.ZombieMania_PlayerState_C|GetCurrentPoints _playerstateref))
  (Variables|Objective|SetObjectivesToBeCompleted (Utilities|Map|MakeMap (Utilities|String|MakeLiteralString "Collect All Weapons") (Variables|Objective|GetCollectedAllWeapons?) (Utilities|String|MakeLiteralString (Utilities|String|Append (Utilities|String|MakeLiteralString "Kill 100 Zombies") " - " (Utilities|String|ToString(Integer) (Variables|Objective|GetTotalZombiesKilled)) "/100")) (>= (Variables|Objective|GetTotalZombiesKilled) 100) (Utilities|String|MakeLiteralString (Utilities|String|Append (Utilities|String|MakeLiteralString "Have 5000 Points") " - " (Utilities|String|ToString(Integer) _currentpoints) "/2000")) (>= _currentpoints 2000))))

(fn AllObjectivesCompleted
  (if (!= (Utilities|Map|Length (Variables|Objective|GetObjectivesToBeCompleted)) 0)
    (CallFunction|AddObjectives)
    (bind _keys (Utilities|Map|Keys (Variables|Objective|GetObjectivesToBeCompleted)))
    (for _array_element _keys
      (if (not (.Value (Utilities|Map|Find (Variables|Objective|GetObjectivesToBeCompleted) _array_element)))
        (LocalVariables|SetLocalIsAllObjectivesCompleted? false)))
    (return (LocalVariables|GetLocalIsAllObjectivesCompleted?))))

(fn GetPlayerDamageAmountBasedonCurrentRound
  (if (> (Variables|Default|GetCurrentRound) 5)
    (if (> (Variables|Default|GetCurrentRound) 10)
      (if (> (Variables|Default|GetCurrentRound) 15)
        (if (> (Variables|Default|GetCurrentRound) 20)
          _
          (else
            _))
        (return 3e+01)
        (else
          (return 15.0)))
      (else
        (return 1e+01)))
    (else
      (return 5.0))))