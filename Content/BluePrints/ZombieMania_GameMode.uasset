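; Game mode for ZombieMania that runs round-based zombie spawning.
; On BeginPlay it caches the game state and all EnemySpawner actors; a one-time flag in Tick also starts a round and ensures the player's main HUD is in the viewport.
; Each round, after a short delay, increments the game state's round and loops a timer that spawns from a random spawner until the zombie count reaches the target.
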(event Custom|SpawnZombies
  (bind _enemyspawners (Variables|Default|GetEnemySpawners))
  (bind _gamestateref (Variables|Default|GetGameStateRef))
  (if (< (Variables|/Game/BluePrints/ZombieMania_GameState.ZombieMania_GameState_C|GetNumberOfZombies _gamestateref) (Variables|/Game/BluePrints/ZombieMania_GameState.ZombieMania_GameState_C|GetNumberOfZombiesToSpawn _gamestateref))
    (Default|SpawnZombie (Utilities|Array|Get(acopy) _enemyspawners (Math|Random|RandomIntegerinRange 0 (- (Utilities|Array|Length _enemyspawners) 1))))
    (else
      (Utilities|Time|ClearandInvalidateTimerbyHandle (stale Custom|StartNewRound _returnvalue)))))

(event Custom|StartNewRound
  (Utilities|FlowControl|Delay 3.0)
  (Default|IncreaseRound (Variables|Default|GetGameStateRef))
  (bind _returnvalue (Utilities|Time|SetTimerbyEvent (delegate Custom|SpawnZombies) 2.5 true)))

(event EventBeginPlay
  (bind _aszombie_mania_game_state (Utilities|Casting|CastToZombieMania_GameState (Game|GetGameState)))
  (Variables|Default|SetGameStateRef _aszombie_mania_game_state)
  (bind _outactors (Actor|GetAllActorsOfClass "/Game/BluePrints/Actors/EnemySpawner.EnemySpawner_C"))
  (Variables|Default|SetEnemySpawners _outactors)
  (if (Variables|Default|GetIsGameStarted?)
    (CallFunction|StartNewRound)))

(event EventTick
  (params (DeltaSeconds :type Float%20%28single-precision%29))
  (if (Variables|Default|GetIsOneTimeInitializerNeeded?)
    (Variables|Default|SetIsOneTimeInitializerNeeded? false)
    (CallFunction|StartNewRound)
    (bind _aszombie_mania_character (Utilities|Casting|CastToZombieMania_Character (Game|Player|GetPlayerPawn 0)))
    (if (not (UserInterface|Viewport|IsinViewport (Variables|/Game/BluePrints/ZombieMania_Character.ZombieMania_Character_C|GetMainHUDRef _aszombie_mania_character)))
      (UserInterface|Viewport|AddtoViewport (Variables|/Game/BluePrints/ZombieMania_Character.ZombieMania_Character_C|GetMainHUDRef _aszombie_mania_character) 0))))

(fn ConstructionScript)