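; Player controller for ZombieMania that handles mouse look and slows it while the character aims with a weapon.
; On BeginPlay it caches the pawn as a ZombieMania_Character and reads the current weapon's aim speed once, defaulting to 1 without one.
; MouseX and MouseY feed yaw and pitch, divided by that cached value when aiming in the matching weapon state.
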(event EventBeginPlay
  (bind _asudemy_character (Utilities|Casting|CastToZombieMania_Character (Game|Player|GetPlayerPawn 0)))
  (bind _output_get (Variables|Default|SetPlayerRef _asudemy_character))
  (if (Utilities|Enum|Equal(Enum) (Variables|/Game/BluePrints/ZombieMania_Character.ZombieMania_Character_C|GethasWeaponEnum _output_get) "NewEnumerator1")
    (Variables|Default|SetAimWeaponSpeed (Variables|/Game/BluePrints/Weapons/BP_WeaponBase.BP_WeaponBase_C|GetAimBasedWeaponSpeed (Variables|/Game/BluePrints/ZombieMania_Character.ZombieMania_Character_C|GetCurrentWeapon (Variables|Default|GetPlayerRef))))
    (else
      (Variables|Default|SetAimWeaponSpeed 1.0))))

(event Input|AxisEvents|InputAxisMouseX
  (params (AxisValue :type Float%20%28single-precision%29))
  (bind _playerref (Variables|Default|GetPlayerRef))
  (Class|PlayerController|AddYawInput (select (and (Variables|/Game/BluePrints/ZombieMania_Character.ZombieMania_Character_C|GetisAiming _playerref) (Utilities|Enum|Equal(Enum) (Variables|/Game/BluePrints/ZombieMania_Character.ZombieMania_Character_C|GethasWeaponEnum _playerref) "NewEnumerator1")) (/ AxisValue (Variables|Default|GetAimWeaponSpeed)) AxisValue)))

(event Input|AxisEvents|InputAxisMouseY
  (params (AxisValue :type Float%20%28single-precision%29))
  (bind _playerref (Variables|Default|GetPlayerRef))
  (Class|PlayerController|AddPitchInput (select (and (Variables|/Game/BluePrints/ZombieMania_Character.ZombieMania_Character_C|GetisAiming _playerref) (Utilities|Enum|Equal(Enum) (Variables|/Game/BluePrints/ZombieMania_Character.ZombieMania_Character_C|GethasWeaponEnum _playerref) "NewEnumerator1")) (/ AxisValue (Variables|Default|GetAimWeaponSpeed)) AxisValue)))

(fn ConstructionScript)